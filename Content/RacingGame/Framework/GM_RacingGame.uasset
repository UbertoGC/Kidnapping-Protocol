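; Game mode for a timed vehicle race, moving through pre-race, countdown, running and win or lose finish.
; On BeginPlay it binds to finish-line checkpoint and point actor crossing events.
; A single timer triggers the out-of-time loss, is re-created to add bonus time, and is cleared on a win.
; Finishing disables input, brakes the vehicle and plays tagged Win/Lose level sequences, though the printed result depends on coin count.
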(event Custom|Game%20Start
  (Development|PrintString "Game has started")
  (bind _returnvalue (Utilities|Time|SetTimerbyEvent (delegate Custom|Lose_OutOfTime) (Variables|Default|GetStartTimerDuration)))
  (Variables|Default|SetTimeRemainingTimer _returnvalue))

(event Custom|Game%20Finish
  (params (Win :type Boolean))
  (bind _returnvalue (Game|Player|GetPlayerPawn 0))
  (bind _assports_car_pawn (Utilities|Casting|CastToSportsCar_Pawn (Game|Player|GetPlayerPawn 0)))
  (Development|PrintString (Utilities|String|SelectString "You win" "You lose" (== (Variables|/Game/VehicleTemplate/Blueprints/SportsCar/SportsCar_Pawn.SportsCar_Pawn_C|GetCoinCount _assports_car_pawn) 6)))
  (Utilities|FlowControl|Sequence
    (:then_0
      (Input|DisableInput _returnvalue (Game|GetPlayerController 0))
      (bind _aswheeled_vehicle_pawn (Utilities|Casting|CastToWheeledVehiclePawn _returnvalue))
      (Class|ChaosVehicleMovementComponent|SetThrottleInput (Variables|/Script/ChaosVehicles.WheeledVehiclePawn|GetVehicleMovementComponent _aswheeled_vehicle_pawn) 0.0)
      (Class|ChaosVehicleMovementComponent|SetHandbrakeInput (Variables|/Script/ChaosVehicles.WheeledVehiclePawn|GetVehicleMovementComponent _aswheeled_vehicle_pawn) true)
      (Class|ChaosVehicleMovementComponent|SetSteeringInput (Variables|/Script/ChaosVehicles.WheeledVehiclePawn|GetVehicleMovementComponent _aswheeled_vehicle_pawn) 1.0)
      (bind _asmotorcycle_pawn (Utilities|Casting|CastToMotorcycle_Pawn (Game|Player|GetPlayerPawn 0)))
      (Audio|Components|Audio|Stop (Variables|/Game/VehicleTemplate/Blueprints/Motorcycle/Motorcycle_Pawn.Motorcycle_Pawn_C|GetSFX_CarEngine _asmotorcycle_pawn)))
    (:then_1
      (bind _outactors (Actor|GetAllActorsOfClass "/Script/LevelSequence.LevelSequenceActor"))
      (for _array_element _outactors
        (if (>= (Utilities|Array|FindItem (Variables|/Script/Engine.Actor|GetTags _array_element) (select Win (Utilities|Name|MakeLiteralName "Win") (Utilities|Name|MakeLiteralName "Lose"))) 0)
          (Sequencer|Player|Play (Variables|/Script/LevelSequence.LevelSequenceActor|GetSequencePlayer _array_element) :!class /Script/MovieScene.MovieSceneSequencePlayer))))))

(event Custom|Start%20Countdown
  (Development|PrintString "Start Countdown")
  (Utilities|FlowControl|Delay (Variables|Default|GetStartCountdownDuration))
  (CallFunction|GameStart))

(event Custom|Lose_OutOfTime
  (bind _output_get (Variables|Default|SetState 2))
  (switch int _output_get
    (:2
      (bind _output_get_2 (Variables|Default|SetWin false))
      (CallFunction|GameFinish _output_get_2))))

(event Custom|Win_CrossTheFinishLine
  (Utilities|Time|ClearandInvalidateTimerbyHandle (Variables|Default|GetTimeRemainingTimer))
  (bind _output_get (Variables|Default|SetState 3))
  (switch int _output_get
    (:3
      (bind _output_get_2 (Variables|Default|SetWin true))
      (CallFunction|GameFinish _output_get_2))))

(event Custom|CrossedACheckpoint
  (params (TimeToAdd :type Integer))
  (CallFunction|AddTimetoTimer TimeToAdd))

(event Custom|PreRace
  (bind _returnvalue (Game|GetPlayerController 0))
  (Development|PrintString "In Pre Race State")
  (Variables|/Script/Engine.PlayerController|SetbShowMouseCursor _returnvalue false)
  (Input|SetInputModeGameOnly _returnvalue false))

(event EventBeginPlay
  (Utilities|FlowControl|Sequence
    (:then_0
      (bind _outactors (Actor|GetAllActorsOfClass "/Game/RacingGame/Checkpoints/BP_Checkpoint.BP_Checkpoint_C"))
      (for _array_element _outactors
        (if (Variables|/Game/RacingGame/Checkpoints/BP_Checkpoint.BP_Checkpoint_C|GetIsFinishLine _array_element)
          (EventDispatchers|BindEventtoOnCheckpointCrossed _array_element (EventDispatchers|CreateEvent :!event Custom|Win_CrossTheFinishLine)))))
    (:then_1
      (bind _outactors_2 (Actor|GetAllActorsOfClass "/Game/RacingGame/Checkpoints/BP_PointActor.BP_PointActor_C"))
      (EventDispatchers|BindEventtoOnCheckpointCrossedwithTime _outactors_2 (EventDispatchers|CreateEvent :!event Custom|CrossedACheckpoint)))
    (:then_2
      (CallFunction|PreRace))))

(fn ConstructionScript)

(fn AddTimetoTimer
  (params (TimeToAdd :type Integer))
  (bind _returnvalue (Utilities|Time|SetTimerbyEvent (EventDispatchers|CreateEvent :!event Custom|Lose_OutOfTime) (+ (Utilities|Time|GetTimerRemainingTimebyHandle (Variables|Default|GetTimeRemainingTimer)) TimeToAdd)))
  (Variables|Default|SetTimeRemainingTimer _returnvalue)
  (Utilities|Casting|CastToVehiclePlayerController (Game|GetPlayerController 0)))