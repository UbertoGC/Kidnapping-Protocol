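; BP_PointActor is a one-shot checkpoint pickup for the racing game that grants time and a coin.
; When any wheeled vehicle overlaps its TriggerBox, it broadcasts OnCheckpointCrossedWithTime with TimeToGive and increments CoinCount on player 0's VehicleAdvPawn, whichever vehicle triggered it.
; If that count equals GM_RacingGame's Complete value, it sets Win and calls WinCrossTheFinishLine.
; It then plays the crossing sound and destroys itself.
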(event OnComponentBeginOverlap(TriggerBox)
  (params (OverlappedComponent :type Primitive%20Component%20Object%20Reference) (OtherActor :type Actor%20Object%20Reference) (OtherComp :type Primitive%20Component%20Object%20Reference) (OtherBodyIndex :type Integer) (bFromSweep :type Boolean) (SweepResult :type Hit%20Result%20Structure%20%28by%20ref%29))
  (Utilities|Casting|CastToWheeledVehiclePawn OtherActor)
  (Default|CallOnCheckpointCrossedwithTime (Variables|Default|GetTime%20to%20give))
  (bind _asvehicle_adv_pawn (Utilities|Casting|CastToVehicleAdvPawn (Game|Player|GetPlayerPawn 0)))
  (bind _output_get (Variables|/Game/VehicleTemplate/Blueprints/SportsCar/SportsCar_Pawn.SportsCar_Pawn_C|SetCoinCount _asvehicle_adv_pawn (+ (Variables|/Game/VehicleTemplate/Blueprints/SportsCar/SportsCar_Pawn.SportsCar_Pawn_C|GetCoinCount _asvehicle_adv_pawn) 1)))
  (bind _returnvalue (Actor|GetActorOfClass "/Game/RacingGame/Framework/GM_RacingGame.GM_RacingGame_C"))
  (if (== (Variables|/Game/RacingGame/Framework/GM_RacingGame.GM_RacingGame_C|GetComplete _returnvalue) _output_get)
    (Variables|/Game/RacingGame/Framework/GM_RacingGame.GM_RacingGame_C|SetWin _returnvalue true)
    (Default|WinCrosstheFinishLine _returnvalue))
  (Audio|PlaySound2D "/Game/RacingGame/Audio/SFX/SFX_CheckpointCrossed.SFX_CheckpointCrossed" 1.0 1.0 0.0 0 0)
  (Actor|DestroyActor))

(fn ConstructionScript)